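; GM_Puzzle, apparently a puzzle game mode, sets up the on-screen widget and serves as a test bed for Hp and Mp values.
; BeginPlay adds BP_Widget to the viewport, prints both values as debug text, then immediately fires CallGMPlayerDie.
; Tick fires CallMyHpUpdate every frame without any change check.
; The Hp increment and threshold-print chains are unconnected and never run.
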(event `self.ReceiveBeginPlay`
  (`KismetSystemLibrary.PrintString` "Hello")
  (bind _returnvalue (`|CreateWidget` "/Game/BP_Widget.BP_Widget_C"))
  (`UserWidget.AddToViewport` _returnvalue 0)
  (`KismetSystemLibrary.PrintString` (`KismetStringLibrary.Conv_IntToString` (`self.hp`)) true true (struct :`G` 0.66 :`B` 1.0 :`A` 1.0) 12.0)
  (`KismetSystemLibrary.PrintString` (`KismetStringLibrary.Conv_IntToString` (`self.mp`)) true true (struct :`G` 0.66 :`B` 1.0 :`A` 1.0) 12.0)
  (`self.GM_Player_Die`))

(event `self.ReceiveTick`
  (params (DeltaSeconds :type "Float (single-precision)"))
  (`self.MyHpUpdate`))

(fn `UserConstructionScript`)